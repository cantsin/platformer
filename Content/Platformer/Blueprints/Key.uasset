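; A platformer key that the player avatar picks up on overlap and carries just in front of it.
; Each tick, while carried and the avatar is not dying, it sweeps to a point ahead of the avatar.
; When the sweep hits a Paper2D sprite, it stays carried only if still overlapping the avatar, so level geometry can knock it loose.
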(event EventBeginPlay)

(event EventActorBeginOverlap
  (params (OtherActor :type Actor%20Object%20Reference))
  ;[1 1 1] Determine if avatar can carry the key.
  (Utilities|Casting|CastToAvatarCharacter OtherActor)
  (Variables|Default|SetisCarried true))

(event EventTick
  (params (DeltaSeconds :type Float%20%28single-precision%29))
  (bind _returnvalue (Game|GetPlayerCharacter 0))
  (bind _returnvalue_2 (Transformation|GetActorLocation))
  (bind _returnvalue_3 (Transformation|GetActorLocation _returnvalue))
  ;[1 1 1] Carry key in front of avatar.
  (bind _asavatar_character (Utilities|Casting|CastToAvatarCharacter _returnvalue)
    (:then
      (if (and (not (Variables|/Game/Platformer/Blueprints/AvatarCharacter.AvatarCharacter_C|GetisDying _asavatar_character)) (Variables|Default|GetisCarried))
        (bind _sweephitresult (Transformation|SetActorLocationAndRotation (Math|Interpolation|VInterpTo _returnvalue_2 (+ (* (Transformation|GetActorForwardVector _returnvalue) 15.0) _returnvalue_3) DeltaSeconds 0.0) (Class|KismetMathLibrary|MakeRot 0.0 0.0 (.Roll (Class|KismetMathLibrary|BreakRot (Math|Rotator|FindLookatRotation _returnvalue_2 _returnvalue_3)))) true))
        (Utilities|Casting|CastToPaperSpriteComponent (.HitComponent (Collision|BreakHitResult _sweephitresult)))
        (Variables|Default|SetisCarried (> (Utilities|Array|Length (Collision|GetOverlappingActors "/Game/Platformer/Blueprints/AvatarCharacter.AvatarCharacter_C" :!class /Script/Engine.Actor)) 0))))
    (:CastFailed
      (Variables|Default|SetisCarried false))))

(fn ConstructionScript)