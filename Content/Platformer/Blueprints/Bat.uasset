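; Bat enemy for a platformer that patrols between two points and instantly kills the player on contact.
; From BeginPlay, a self-calling Loop event eases the capsule to BeginningPosition and EndingPosition in turn, flipping the actor 180 degrees after each leg.
; The Hit event destroys an AvatarCharacter when the hit is blocking and its time falls within a small threshold.
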(event Custom|Loop
  ;[1 1 1] Patrol.
  (Components|MoveComponentTo (Variables|Collision|GetCapsuleComponent) (Variables|Default|GetbeginningPosition) "0.000000,0.000000,0.000000" true true 3.0)
  (Transformation|SetActorRelativeRotation "0,180.000000, 0")
  (Components|MoveComponentTo (Variables|Collision|GetCapsuleComponent) (Variables|Default|GetendingPosition) "0.000000,180.000000,0.000000" true true 3.0)
  (Transformation|SetActorRelativeRotation "0,0.000000, 0")
  (CallFunction|Loop))

(event EventBeginPlay
  ;[1 1 1] Patrol.
  (Components|MoveComponentTo (Variables|Collision|GetCapsuleComponent) (Variables|Default|GetbeginningPosition) "0.000000,0.000000,0.000000" true true 3.0)
  (Transformation|SetActorRelativeRotation "0,180.000000, 0")
  (Components|MoveComponentTo (Variables|Collision|GetCapsuleComponent) (Variables|Default|GetendingPosition) "0.000000,180.000000,0.000000" true true 3.0)
  (Transformation|SetActorRelativeRotation "0,0.000000, 0")
  (CallFunction|Loop))

(event EventActorBeginOverlap
  (params (OtherActor :type Actor%20Object%20Reference)))

(event EventTick
  (params (DeltaSeconds :type Float%20%28single-precision%29)))

(event EventDestroyed
  (Utilities|FlowControl|Delay 0.2))

(event EventHit
  (params (MyComp :type Primitive%20Component%20Object%20Reference) (Other :type Actor%20Object%20Reference) (OtherComp :type Primitive%20Component%20Object%20Reference) (bSelfMoved :type Boolean) (HitLocation :type Vector :default "0, 0, 0") (HitNormal :type Vector :default "0, 0, 0") (NormalImpulse :type Vector :default "0, 0, 0") (Hit :type Hit%20Result%20Structure%20%28by%20ref%29))
  (bind (_bblockinghit _time) (Collision|BreakHitResult Hit))
  ;[1 1 1] Instakill.
  (bind _asavatar_character (Utilities|Casting|CastToAvatarCharacter Other))
  (if (and _bblockinghit (<= _time 0.2))
    (Actor|DestroyActor _asavatar_character)))

(fn ConstructionScript)