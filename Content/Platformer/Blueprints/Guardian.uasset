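; Guardian is a 2D platformer enemy that destroys any AvatarCharacter hitting its capsule and shoots Fireballs on sight.
; Each Tick, a short line trace along negative X looks for Pawn or WorldDynamic objects and switches between idle and attack flipbooks.
; The IsShooting flag lets the first shot fire immediately, then a Delay on Tick throttles further shots and another delays the flag's reset.
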(event OnComponentHit(CapsuleComponent)
  (params (OtherActor :type Actor%20Object%20Reference) (OtherComp :type Primitive%20Component%20Object%20Reference) (NormalImpulse :type Vector :default "0, 0, 0") (Hit :type Hit%20Result%20Structure%20%28by%20ref%29))
  ;[1 1 1] Instakill.
  (bind _asavatar_character (Utilities|Casting|CastToAvatarCharacter OtherActor))
  (Actor|DestroyActor _asavatar_character))

(event EventTick
  (params (DeltaSeconds :type Float%20%28single-precision%29))
  ;[1 1 1] Shoot upon sight.
  (bind _returnvalue (Collision|LineTraceForObjects (- (Transformation|GetActorLocation) "0.000000,0.000000,4.000000") (- (Transformation|GetActorLocation) "300.000000, 0,4.000000") (Utilities|Array|MakeArray "ObjectTypeQuery3" "ObjectTypeQuery2") false 0 "None"))
  (if _returnvalue
    (Sprite|SetFlipbook "/Game/Platformer/Flipbooks/GuardianAttack.GuardianAttack")
    (if (Variables|Default|GetisShooting)
      ;[1 1 1] Shoot to kill.
      (Utilities|FlowControl|Delay 1.5)
      (else
        (Variables|Default|SetisShooting true)))
    (Game|SpawnActorfromClass "/Game/Platformer/Blueprints/Fireball.Fireball_C" (Math|Transform|MakeTransform (+ (Transformation|GetWorldLocation (Variables|Collision|GetCapsuleComponent)) "-10.000000,0.000000,-2.000000") (Class|KismetMathLibrary|MakeRot 0.0 0.0 1.8e+02)) false 0)
    (else
      (Sprite|SetFlipbook "/Game/Platformer/Flipbooks/Guardian.Guardian")
      (Utilities|FlowControl|Delay 1.5)
      (Variables|Default|SetisShooting false))))

(fn ConstructionScript)