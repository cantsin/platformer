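; Platformer game mode that respawns the player's avatar character after it is destroyed.
; On BeginPlay it binds to the player character's OnDestroyed event.
; When that fires, it waits briefly, spawns a new AvatarCharacter at SpawnLocation, has the first player controller possess it, then calls Respawn to rebind the event for the next death.
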(event Custom|OnDestroyed_Event
  ;[1 1 1] Respawn.
  (Utilities|FlowControl|Delay 2.0)
  (bind _returnvalue (Game|SpawnActorfromClass "/Game/Platformer/Blueprints/AvatarCharacter.AvatarCharacter_C" (Variables|Default|GetSpawn%20Location) false 0))
  (Pawn|Possess (Game|GetPlayerController 0) _returnvalue)
  (CallFunction|Respawn))

(event Custom|Respawn
  ;[1 1 1] Respawn.
  (bind _asavatar_character (Utilities|Casting|CastToAvatarCharacter (Game|GetPlayerCharacter 0)))
  (Game|BindEventtoOnDestroyed _asavatar_character (delegate Custom|OnDestroyed_Event)))

(event EventBeginPlay
  ;[1 1 1] Respawn.
  (bind _asavatar_character (Utilities|Casting|CastToAvatarCharacter (Game|GetPlayerCharacter 0)))
  (Game|BindEventtoOnDestroyed _asavatar_character (delegate Custom|OnDestroyed_Event)))

(fn ConstructionScript)