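; ChestKey is a key actor that the player avatar picks up and carries in a platformer.
; Overlap with an AvatarCharacter sets the carried flag.
; While carried and the avatar is not dying, Tick interpolates the key toward a point just in front of the avatar and turns it to face them.
; A failed player cast on Tick clears the flag.
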(event EventBeginPlay)

(event EventActorBeginOverlap
  (params (OtherActor :type Actor%20Object%20Reference))
  ;[1 1 1] Determine if avatar can carry the key.
  (Utilities|Casting|CastToAvatarCharacter OtherActor)
  (Variables|Default|SetisCarried true))

(event EventTick
  (params (DeltaSeconds :type Float%20%28single-precision%29))
  (bind _returnvalue (Game|GetPlayerCharacter 0))
  (bind _returnvalue_2 (Transformation|GetActorLocation))
  (bind _returnvalue_3 (Transformation|GetActorLocation _returnvalue))
  ;[1 1 1] Carry key in front of avatar.
  (bind _asavatar_character (Utilities|Casting|CastToAvatarCharacter _returnvalue)
    (:then
      (if (and (not (Variables|/Game/Platformer/Blueprints/AvatarCharacter.AvatarCharacter_C|GetisDying _asavatar_character)) (Variables|Default|GetisCarried))
        (Transformation|SetActorLocationAndRotation (Math|Interpolation|VInterpTo _returnvalue_2 (+ (* (Transformation|GetActorForwardVector _returnvalue) 15.0) _returnvalue_3) DeltaSeconds 0.0) (Math|Rotator|FindLookatRotation _returnvalue_2 _returnvalue_3))))
    (:CastFailed
      (Variables|Default|SetisCarried false))))

(event EventHit
  (params (MyComp :type Primitive%20Component%20Object%20Reference) (Other :type Actor%20Object%20Reference) (OtherComp :type Primitive%20Component%20Object%20Reference) (bSelfMoved :type Boolean) (HitLocation :type Vector :default "0, 0, 0") (HitNormal :type Vector :default "0, 0, 0") (NormalImpulse :type Vector :default "0, 0, 0") (Hit :type Hit%20Result%20Structure%20%28by%20ref%29))
  ;[1 1 1] Determine if avatar can carry the key.
)

(fn ConstructionScript)