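; Player avatar for a 2D side-scrolling platformer, with running, jumping by key or touch, and ladder climbing.
; Trigger volumes tagged "ladder" allow climbing, which uses Flying movement until overlap ends; Tick clears the ability outside volumes.
; Movement input drives flipbook choice and facing through controller yaw, flipped on a delay to animate climbing.
; BeginPlay records the spawn transform in the GameMode; EndPlay leaves an AvatarDeath corpse, and R self-destructs.
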(event Custom|UpdateAnimation
  (bind _returnvalue (Pawn|GetController))
  ;[1 1 1] Animation.
  (if (Variables|Default|GetisClimbing)
    (Sprite|SetFlipbook (Variables|Default|GetSprite) "/Game/Platformer/Flipbooks/AvatarClimb.AvatarClimb")
    ;[1 1 1] Climbing animation.
    (Utilities|FlowControl|Delay 0.2)
    (if (!= (.Z (Math|Vector|BreakVector (Transformation|GetVelocity))) 0.0)
      (Pawn|SetControlRotation _returnvalue (Class|KismetMathLibrary|MakeRot 0.0 (Math|Float|%(Float) (+ (.Yaw (Class|KismetMathLibrary|BreakRot (Pawn|GetControlRotation _returnvalue :!class /Script/Engine.Controller))) 1.8e+02) 3.6e+02) 0.0)))
    (elif (or (Variables|Default|GetisRunning) (> (.X (Math|Vector|BreakVector (Transformation|GetVelocity))) 0.0))
      (Sprite|SetFlipbook (Variables|Default|GetSprite) "/Game/Platformer/Flipbooks/AvatarRun.AvatarRun")
      (else
        (Sprite|SetFlipbook (Variables|Default|GetSprite) "/Game/Platformer/Flipbooks/AvatarIdle.AvatarIdle")))))

(event EventEndPlay
  (params (EndPlayReason :type EEndPlayReason%20Enum :default "ActorDestroyed"))
  ;[1 1 1] Leave a corpse.
  (Game|SpawnActorfromClass "/Game/Platformer/Blueprints/AvatarDeath.AvatarDeath_C" (Math|Conversions|ToTransform(Vector) (Transformation|GetActorLocation)) true 8.0 0))

(event EventTick
  (params (DeltaSeconds :type Float%20%28single-precision%29))
  ;[1 1 1] Hack to stop climbing when not intersecting any volume.
  (if (== (Utilities|Array|Length (Collision|GetOverlappingActors "/Script/Engine.TriggerVolume" :!class /Script/Engine.PrimitiveComponent)) 0)
    (Variables|Default|SetcanClimb false)))

(event EventBeginPlay
  ;[1 1 1] Transform.
  (bind _asgame_mode (Utilities|Casting|CastToGameMode (Game|GetGameMode)))
  (Variables|/Game/Platformer/Blueprints/GameMode.GameMode_C|SetSpawn%20Location _asgame_mode (Transformation|GetActorTransform)))

(event EventActorBeginOverlap
  (params (OtherActor :type Actor%20Object%20Reference))
  ;[1 1 1] Climbing ability.
  (bind _astrigger_volume (Utilities|Casting|CastToTriggerVolume OtherActor))
  (Variables|Default|SetcanClimb (Components|ComponentHasTag _astrigger_volume "ladder")))

(event EventActorEndOverlap
  (params (OtherActor :type Actor%20Object%20Reference))
  (bind _charactermovement (Variables|Character|GetCharacterMovement))
  ;[1 1 1] Climbing ability.
  (bind _astrigger_volume (Utilities|Casting|CastToTriggerVolume OtherActor))
  (Variables|Default|SetisClimbing false)
  (switch Utilities|FlowControl|Switch|SwitchonEMovementMode (Variables|/Script/Engine.CharacterMovementComponent|GetMovementMode _charactermovement)
    (:MOVE_Flying
      (Pawn|Components|CharacterMovement|SetMovementMode _charactermovement "MOVE_Walking" 0)
      (Variables|Default|SetcanClimb false))))

(event Input|ActionEvents|InputActionJump
  ;[1 1 1] Jump.
  (:Pressed
    (Character|Jump)
    (Variables|Default|SetisJumping true))
  (:Released
    (Character|StopJumping)
    (Variables|Default|SetisJumping false)))

(event Input|AxisEvents|InputAxisClimb
  (params (AxisValue :type Float%20%28single-precision%29))
  ;[1 1 1] Start climbing.
  (Pawn|Input|AddMovementInput "0.000000,0.000000,1.000000" AxisValue false))

(event Input|AxisEvents|InputAxisMoveRight
  (params (AxisValue :type Float%20%28single-precision%29))
  ;[1 1 1] Movement.
  (Pawn|Input|AddMovementInput "1.000000, 0, 0" AxisValue false)
  (CallFunction|UpdateAnimation)
  (Math|Float|CompareFloat AxisValue 0.0
    (:>
      (Pawn|SetControlRotation (Pawn|GetController) (Class|KismetMathLibrary|MakeRot 0.0 0.0 0.0))
      (Variables|Default|SetisRunning true))
    (:==
      (Variables|Default|SetisRunning false))
    (:<
      (Pawn|SetControlRotation (Pawn|GetController) (Class|KismetMathLibrary|MakeRot 0.0 1.8e+02 0.0))
      (Variables|Default|SetisRunning true))))

(event Input|KeyboardEvents|R
  ;[1 1 1] Suicide.
  (:Pressed
    (Actor|DestroyActor)))

(event Input|KeyboardEvents|Up
  ;[1 1 1] Start climbing.
  (:Pressed
    (if (Variables|Default|GetcanClimb)
      (Pawn|Components|CharacterMovement|SetMovementMode (Variables|Character|GetCharacterMovement) "MOVE_Flying" 0)
      (Variables|Default|SetisClimbing true)
      (Sprite|SetFlipbook (Variables|Default|GetSprite) "/Game/Platformer/Flipbooks/AvatarClimb.AvatarClimb"))))

(event Input|TouchEvents|InputTouch
  (params (Location :type Vector) (FingerIndex :type ETouchIndex%20Enum))
  ;[1 1 1] Jump.
  (:Pressed
    (Character|Jump)
    (Variables|Default|SetisJumping true))
  (:Released
    (Character|StopJumping)
    (Variables|Default|SetisJumping false)))

(fn ConstructionScript)