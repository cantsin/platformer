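; PlatformHUD is the HUD for a platformer escape game, drawing on-screen text messages in the Alagard font.
; BeginPlay sets an Introduction flag and clears it after a short delay, during which DrawHUD shows an opening taunt.
; Afterwards, DrawHUD casts the player character to AvatarCharacter and shows a victory message whenever its HasWon flag is set.
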(event EventActorBeginOverlap
  (params (OtherActor :type Actor%20Object%20Reference)))

(event EventTick
  (params (DeltaSeconds :type Float%20%28single-precision%29)))

(event EventDrawHUD
  (params (SizeX :type Integer) (SizeY :type Integer))
  ;[1 1 1] Introduction.
  (if (Variables|Default|Getintroduction)
    (HUD|DrawText (HUD|GetHUD (Game|GetPlayerController 0)) "Escape...if you can!" "(R=1.000000,G=1.000000,B=1.000000,A=1.000000)" 5e+01 5.0 "/Game/Platformer/Fonts/Alagard.Alagard" 1.0 false)
    (else
      ;[1 1 1] Victory message.
      (bind _asavatar_character (Utilities|Casting|CastToAvatarCharacter (Game|GetPlayerCharacter 0)))
      (if (Variables|/Game/Platformer/Blueprints/AvatarCharacter.AvatarCharacter_C|GethasWon _asavatar_character)
        (HUD|DrawText (HUD|GetHUD (Game|GetPlayerController 0)) "Congratulations! You escaped!" "(R=1.000000,G=1.000000,B=1.000000,A=1.000000)" 5e+01 5.0 "/Game/Platformer/Fonts/Alagard.Alagard" 1.0 false)))))

(event EventBeginPlay
  ;[1 1 1] Set introduction time length.
  (Variables|Default|Setintroduction true)
  (Utilities|FlowControl|Delay 5.0)
  (Variables|Default|Setintroduction false))

(fn ConstructionScript)