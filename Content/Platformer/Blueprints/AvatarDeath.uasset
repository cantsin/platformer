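; AvatarDeath is a temporary Paper2D actor for the dead avatar that destroys itself once its TimeToLast delay elapses.
; Overlapping a KillZVolume eases its flipbook over one second to a new relative location.
; That target takes X and Z from the actor's world location and Y from the volume brush's box extent, not its position.
; Tick and the construction script are empty, and some disconnected nodes remain.
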(event EventTick
  (params (DeltaSeconds :type Float%20%28single-precision%29)))

(event EventActorBeginOverlap
  (params (OtherActor :type Actor%20Object%20Reference))
  (bind _paperflipbook (Variables|Default|GetPaperFlipbook))
  (bind _returnvalue (Components|GetOwner _paperflipbook))
  (bind _returnvalue_2 (Transformation|GetActorLocation _returnvalue))
  (bind (_x _y _z) (Math|Vector|BreakVector _returnvalue_2))
  (bind _askill_zvolume (Utilities|Casting|CastToKillZVolume OtherActor))
  (Components|MoveComponentTo _paperflipbook (Math|Vector|MakeVector _x (.Y (Math|Vector|BreakVector (.BoxExtent (Collision|GetComponentBounds (Variables|/Script/Engine.Brush|GetBrushComponent _askill_zvolume))))) _z) "0, 0, 0" true true 1.0))

(event EventBeginPlay
  ;[1 1 1] Destroy dead avatar after a while.
  (Utilities|FlowControl|Delay (Variables|Default|GetTimeToLast))
  (Actor|DestroyActor))

(fn ConstructionScript)